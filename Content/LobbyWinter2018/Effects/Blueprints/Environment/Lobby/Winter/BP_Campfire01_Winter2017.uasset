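; BP_Campfire01_Winter2017 is a campfire environment prop for the Winter lobby that animates the brightness of its firelight.
; On BeginPlay a timeline's Brightness track drives three spot lights, including a volumetric one, each with its own scale and base intensity.
; An async Campfire bank load is present but unconnected, and its loaded callback is empty.
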(event `self.ReceiveBeginPlay`
  (bind (_direction _brightness) (`Timeline|Timeline_0` :!via `PlayFromStart`)
    (:`Update`
      (`LightComponent.SetIntensity` (`self.SpotLight_LF`) (+ (* _brightness 20000.0) 10000.0))
      (`LightComponent.SetIntensity` (`self.Camp_SpotLight`) (+ (* _brightness 2000.0) 1000.0))
      (`LightComponent.SetIntensity` (`self.SpotLight_LF_Volumetric`) (+ (* _brightness 400.0) 200.0)))))

(event `OnBankLoaded`
  (params (Result :type "EAkResult Enum" :default "NotImplemented")))

(fn `UserConstructionScript`)