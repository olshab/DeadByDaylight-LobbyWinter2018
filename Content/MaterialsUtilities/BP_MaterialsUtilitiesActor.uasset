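; BP_MaterialsUtilitiesActor is an actor that hosts the materials utilities UI for its static mesh.
; On BeginPlay it creates WBP_MaterialsUtilities, adds it to the viewport and assigns it the StaticMesh component.
; It then resets the actor transform to identity and prints the root and mesh world transforms for debugging.
; An alternative transform call is left unconnected, and the construction script is empty.
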(event `self.ReceiveBeginPlay`
  (bind _returnvalue (`|CreateWidget` "/Game/MaterialsUtilities/WBP_MaterialsUtilities.WBP_MaterialsUtilities_C"))
  (`UserWidget.AddToViewport` _returnvalue 0)
  (`/Game/MaterialsUtilities/WBP_MaterialsUtilities.AssignMesh` _returnvalue (`self.StaticMesh`))
  (`self.K2_SetActorTransform` (`KismetMathLibrary.MakeTransform` (0.0 0.0 0.0) (struct) (1.0 1.0 1.0)))
  (`/Game/LoggingUtilities/BlueprintLoggingLibrary.PrintString` (`KismetStringLibrary.Conv_TransformToString` (`SceneComponent.K2_GetComponentToWorld` (`self.DefaultSceneRoot`))) "NewEnumerator0" "LogBlueprintUserMessages" true self)
  (`/Game/LoggingUtilities/BlueprintLoggingLibrary.PrintString` (`KismetStringLibrary.Conv_TransformToString` (`SceneComponent.K2_GetComponentToWorld` (`self.StaticMesh`))) "NewEnumerator2" "LogBlueprintUserMessages" true self))

(fn `UserConstructionScript`)